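; Player character for a side-view 2D game, moving along the world X axis with flipbook sprite animation.
; On BeginPlay it adds its Enhanced Input mapping context to the first player's input subsystem.
; The move action applies movement input and sets the walk flipbook, switching back to the default flipbook on completion.
; Each tick, the sign of X velocity rotates the sprite to face the direction of travel, keeping its last facing when stopped.
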(event `self.ReceiveBeginPlay`
  (bind _returnvalue (pcsubsystem `EnhancedInputLocalPlayerSubsystem` (`GameplayStatics.GetPlayerController` 0)))
  (`/Engine/EditorBlueprintResources/StandardMacros.IsValid` _returnvalue
    (:`Is Valid`
      (`EnhancedInputSubsystemInterface.AddMappingContext` _returnvalue "/Game/ThomasContent/Blueprints/IMC_ThomasClark_CharacterInput.IMC_ThomasClark_CharacterInput" 0 (struct)))))

(event `self.ReceiveTick`
  (params (DeltaSeconds :type "Float (single-precision)"))
  (`self.UpdateCharacterRotation`))

(event `UpdateCharacterRotation`
  (bind _sprite (`self.Sprite`))
  (bind _velocity_x (`KismetMathLibrary.BreakVector` (`MovementComponent.Velocity` (`self.CharacterMovement`))))
  (`/Engine/EditorBlueprintResources/StandardMacros.CompareFloat` _velocity_x
    (:`>`
      (`SceneComponent.K2_SetRelativeRotation` _sprite (struct) false false))
    (:`<`
      (`SceneComponent.K2_SetRelativeRotation` _sprite (struct :`Yaw` 180.0) false false))))

(event `EnhancedInput|/Game/ThomasContent/Blueprints/IA_ThomasClark_Move`
  (params (ActionValue :type "Float (double-precision)") (ElapsedSeconds :type "Float (double-precision)") (TriggeredSeconds :type "Float (double-precision)") (InputAction :type "InputAction Object Reference" :default "/Game/ThomasContent/Blueprints/IA_ThomasClark_Move.IA_ThomasClark_Move"))
  (:`Triggered`
    (`self.AddMovementInput` (1.0 0.0 0.0) ActionValue)
    (`PaperFlipbookComponent.SetFlipbook` (`self.Sprite`) "/Game/ThomasContent/Flipbooks/F_LargeFellaWalk.F_LargeFellaWalk"))
  (:`Completed`
    (`PaperFlipbookComponent.SetFlipbook` (`self.Sprite`) "/Game/ThomasContent/Flipbooks/FB_LargeFella.FB_LargeFella")))

(fn `UserConstructionScript`)